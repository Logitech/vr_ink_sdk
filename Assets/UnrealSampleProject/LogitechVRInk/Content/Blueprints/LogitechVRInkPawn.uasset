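; VR pawn that detects a Logitech VR Ink stylus among its motion controllers and gives it the matching model.
; On BeginPlay it sets a floor tracking origin and waits briefly for SteamVR to initialize.
; It then tests the right and left controllers with IsVRInk, spawning a LogitechVRInk actor snapped to each one that matches.
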(event `self.ReceiveBeginPlay`
  (bind _mc_right (`self.MC_Right`))
  (bind _mc_left (`self.MC_Left`))
  (`HeadMountedDisplayFunctionLibrary.SetTrackingOrigin` "Floor")
  (`KismetSystemLibrary.Delay` 0.2) ; You need to use a Delay becasue it takles a couple of frame for SteamVR To initialize at start up
  (`|ExecutionSequence`
    (:`then_0`
      ;[1 1 1] Dettect which Motion Controller is the VR Ink and instantiate the Logitech VR Ink model on the correct MC
      (bind _returnvalue (`LogitechVRInkLibrary.IsVRInk` _mc_right))
      (if _returnvalue
        (bind _returnvalue_2 (`|SpawnActorFromClass` (`self.LogitechVRInk`) (`SceneComponent.GetRelativeTransform` _mc_right) "Undefined" "OverrideRootScale" null null))
        (`self.K2_AttachToComponent` _returnvalue_2 (`self.MC_Right`) "None" "SnapToTarget" "SnapToTarget" "SnapToTarget" true)))
    (:`then_1`
      (bind _returnvalue_3 (`LogitechVRInkLibrary.IsVRInk` _mc_left))
      (if _returnvalue_3
        (bind _returnvalue_4 (`|SpawnActorFromClass` (`self.LogitechVRInk`) (`SceneComponent.GetRelativeTransform` _mc_left) "Undefined" "OverrideRootScale" null null))
        (`self.K2_AttachToComponent` _returnvalue_4 (`self.MC_Left`) "None" "SnapToTarget" "SnapToTarget" "SnapToTarget" true)))))

(fn `UserConstructionScript`)